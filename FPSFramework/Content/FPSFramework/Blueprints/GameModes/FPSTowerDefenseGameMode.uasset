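; Game mode for the tower defense mode that kicks off enemy waves when play begins.
; On BeginPlay it finds and caches the level's BP_GridManager and BP_SpawnerManager actors, then after a short delay calls StartGame, which tells the spawner manager to begin a wave.
; It exposes the cached grid manager to other objects through an IGetGridManager getter.
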(event `self.ReceiveBeginPlay`
  (bind _returnvalue (`GameplayStatics.GetActorOfClass` "/Game/FPSFramework/Blueprints/Grid/BP_GridManager.BP_GridManager_C"))
  (set `self.GridManager` _returnvalue)
  (bind _returnvalue_2 (`GameplayStatics.GetActorOfClass` "/Game/FPSFramework/Blueprints/BP_SpawnerManager.BP_SpawnerManager_C"))
  (set `self.SpawnerManager` _returnvalue_2)
  (`KismetSystemLibrary.Delay` 0.2)
  (`self.StartGame`))

(event `StartGame`
  (`/Game/FPSFramework/Blueprints/BP_SpawnerManager.BeginWave` (`self.SpawnerManager`)))

(fn `I_GetGridManager`
  (returns (GridManager :type "/Game/FPSFramework/Blueprints/Grid/BP_GridManager Object Reference"))
  (return (`self.GridManager`)))

(fn `UserConstructionScript`)