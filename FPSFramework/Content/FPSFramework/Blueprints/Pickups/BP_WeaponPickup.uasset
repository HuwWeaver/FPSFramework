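; BP_WeaponPickup is a pickup actor that offers a random weapon from the WeaponsData table.
; On BeginPlay it picks a random row name and sets the skeletal mesh to that row's cosmetic mesh.
; Any actor overlapping the Box receives the weapon name through the ChangeWeapon interface message, after which the pickup immediately rerolls to another random weapon.
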(event `self.ReceiveBeginPlay`
  (`parent.ReceiveBeginPlay`)
  (bind _outrownames (`DataTableFunctionLibrary.GetDataTableRowNames` "/Game/FPSFramework/Blueprints/Weapons/WeaponsData.WeaponsData" :!label _label))
  (bind _output_get (set `self.WeaponToSpawn` (`KismetArrayLibrary.Array_Random` _outrownames)))
  (bind _returnvalue (`|GetDataTableRow` "/Game/FPSFramework/Blueprints/Weapons/WeaponsData.WeaponsData" _output_get)
    (:`then`
      (`SkinnedMeshComponent.SetSkinnedAssetAndUpdate` (`self.SkeletalMesh`) (`.SkeleMesh_4_5C12C40B4E44497C4CA002AEAC24959B` (break `/Game/FPSFramework/Structs/WpnCosmeticsStruct` (`.CosmeticProperties_28_7D9154E7427EC37259C88C9C3DAB187E` (break `/Game/FPSFramework/Structs/FullWpnPropertiesStruct` _returnvalue)))) true))))

(event `RefreshWeapon`
  (goto _label))

(event `self.Box.OnComponentBeginOverlap`
  (params (OverlappedComponent :type "PrimitiveComponent Object Reference") (OtherActor :type "Actor Object Reference") (OtherComp :type "PrimitiveComponent Object Reference") (OtherBodyIndex :type Integer) (bFromSweep :type Boolean) (SweepResult :type "HitResult Structure (by ref)"))
  (message `/Game/FPSFramework/Blueprints/Characters/Player/BPI_Inventory.I_ChangeWeapon` OtherActor (`self.WeaponToSpawn`))
  (`self.RefreshWeapon`))

(fn `UserConstructionScript`
  (`parent.UserConstructionScript`))