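; BP_GridManager builds and maintains a grid of BP_GridNode actors, with node types for empty, wall and tower cells.
; On BeginPlay it clears existing nodes, then spawns a rotated, evenly spaced grid, flags entrance/exit cells and maps coordinates to nodes in GridRef.
; UpdateNode looks up a node's coordinates and swaps in a new actor by type.
; Only Wall has its own class; tower types currently spawn the base node.
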(event `self.ReceiveBeginPlay`
  (`self.CreateGrid`))

(event `ClearGrid`
  (bind _gridref (`self.GridRef`))
  ;[1 1 1] Clear Grid
  (`KismetSystemLibrary.PrintString` "Clearing Grid Nodes..")
  (bind _values (`BlueprintMapLibrary.Map_Values` _gridref))
  (for _array_element _values
    (`self.K2_DestroyActor` _array_element))
  (`BlueprintMapLibrary.Map_Clear` _gridref)
  (bind _outactors (`GameplayStatics.GetAllActorsOfClass` "/Game/FPSFramework/Blueprints/Grid/BP_GridNode.BP_GridNode_C"))
  (for _array_element_2 _outactors
    (`self.K2_DestroyActor` _array_element_2))
  (`KismetSystemLibrary.PrintString` "Grid Cleared!"))

(event `CreateGrid`
  (bind (_returnvalue_location _returnvalue_rotation) (`KismetMathLibrary.BreakTransform` (`self.GetTransform`)))
  ;[1 1 1] Create Grid
  (`self.ClearGrid`)
  (`KismetSystemLibrary.PrintString` "Creating Grid...")
  (for _index (range (`self.NumColumns`))
    (for _index_2 (range (`self.NumRows`))
      (bind _gridcoordinatesstruct (make `/Game/FPSFramework/Blueprints/Structs/GridCoordinatesStruct` _index _index_2))
      (bind _returnvalue (`|SpawnActorFromClass` "/Game/FPSFramework/Blueprints/Grid/BP_GridNode.BP_GridNode_C" (`KismetMathLibrary.MakeTransform` (+ _returnvalue_location (`KismetMathLibrary.GreaterGreater_VectorRotator` (`KismetMathLibrary.MakeVector` (* _index_2 500.0) (* _index 500.0)) _returnvalue_rotation)) _returnvalue_rotation) "Undefined" "OverrideRootScale" null (`KismetArrayLibrary.Array_Contains` (`self.EntrancesAndExits`) _gridcoordinatesstruct) null))
      (`BlueprintMapLibrary.Map_Add` (`self.GridRef`) _gridcoordinatesstruct _returnvalue)
      (`/Game/FPSFramework/Blueprints/Grid/BP_GridNode.SetCoords` _returnvalue _gridcoordinatesstruct)))
  (`KismetSystemLibrary.PrintString` "Grid Created!"))

(event `UpdateNode`
  (params (NodeToUpdate :type "/Game/FPSFramework/Blueprints/Grid/BP_GridNode Object Reference") (NewType :type "/Game/FPSFramework/Blueprints/Enumns/EGridNodeTypes Enum" :default "NewEnumerator0"))
  (bind _gridref (`self.GridRef`))
  (bind _cachedgridref (`self.CachedGridRef`))
  (bind _value (`BlueprintMapLibrary.Map_Find` _gridref _cachedgridref))
  (bind (_returnvalue_location _returnvalue_rotation) (`KismetMathLibrary.BreakTransform` (`self.GetTransform` _value)))
  ;[1 1 1] Update/Replace Grid Node
  (bind _keys (`BlueprintMapLibrary.Map_Keys` (`self.GridRef`)))
  (for _array_element _keys
    (bind (_value_2 _returnvalue) (`BlueprintMapLibrary.Map_Find` (`self.GridRef`) _array_element))
    (if _returnvalue
      (if (== NodeToUpdate _value_2)
        (bind (_x _y) (break `/Game/FPSFramework/Blueprints/Structs/GridCoordinatesStruct` _array_element))
        (setmembers `/Game/FPSFramework/Blueprints/Structs/GridCoordinatesStruct` :`StructRef` (`self.CachedGridRef`) :`X` _x :`Y` _y)
        (break))))
  (bind _returnvalue_2 (`|SpawnActorFromClass` (select `/Game/FPSFramework/Blueprints/Enumns/EGridNodeTypes` NewType :`NewEnumerator0` "/Game/FPSFramework/Blueprints/Grid/BP_GridNode.BP_GridNode_C" :`NewEnumerator1` "/Game/FPSFramework/Blueprints/Grid/BP_GridWall.BP_GridWall_C" :`NewEnumerator2` "/Game/FPSFramework/Blueprints/Grid/BP_GridNode.BP_GridNode_C" :`NewEnumerator3` "/Game/FPSFramework/Blueprints/Grid/BP_GridNode.BP_GridNode_C" :`NewEnumerator4` "/Game/FPSFramework/Blueprints/Grid/BP_GridNode.BP_GridNode_C" :!type "Actor Class Reference") (`KismetMathLibrary.MakeTransform` _returnvalue_location _returnvalue_rotation) "Undefined" "OverrideRootScale" null null))
  (`self.K2_DestroyActor` _value)
  (bind _asbp_grid_node (cast `/Game/FPSFramework/Blueprints/Grid/BP_GridNode` _returnvalue_2))
  (`BlueprintMapLibrary.Map_Add` _gridref _cachedgridref _asbp_grid_node)
  (`/Game/FPSFramework/Blueprints/Grid/BP_GridNode.SetCoords` _asbp_grid_node _cachedgridref))

(fn `UserConstructionScript`)