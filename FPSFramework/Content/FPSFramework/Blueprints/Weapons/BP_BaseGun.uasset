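; Base gun Blueprint for the FPS framework, configured on init from a weapons data table row and driven through interface calls.
; Single, burst and auto fire modes, the latter two timer-looped, check magazine ammo then fire pellets as single traces, multi traces or projectiles.
; Shots aim from screen center within an inaccuracy cone scaled by ADS, then apply recoil and FX.
; Ammo and fire mode changes notify the owner's HUD through interface messages.
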(event `/Game/FPSFramework/Blueprints/Weapons/BPI_Weapons.I_DeinitWeapon`
  ;[1 1 1] Deinit
)

(event `/Game/FPSFramework/Blueprints/Weapons/BPI_Weapons.I_InitWeapon`
  (params (WeaponDataRef :type Name))
  ;[1 1 1] INIT
  (`|ExecutionSequence`
    (:`then_0`
      (bind _returnvalue (`|GetDataTableRow` "/Game/FPSFramework/Blueprints/Weapons/WeaponsData.WeaponsData" WeaponDataRef)
        (:`then`
          (set `self.WeaponProperties` _returnvalue))
        (:`RowNotFound`
          (`KismetSystemLibrary.PrintString` (`KismetStringLibrary.Concat_StrStr` "Row Not Found in Weapons Data Table - giving player copy of first weapon in Data Table. Row name given: " (`KismetStringLibrary.Conv_NameToString` WeaponDataRef)) true true (struct :`R` 1.0 :`G` 0.005584 :`A` 1.0))
          (bind _outrownames (`DataTableFunctionLibrary.GetDataTableRowNames` "/Game/FPSFramework/Blueprints/Weapons/WeaponsData.WeaponsData"))
          (`|GetDataTableRow` "/Game/FPSFramework/Blueprints/Weapons/WeaponsData.WeaponsData" (`|GetArrayItem` _outrownames)))))
    (:`then_1`
      (`self.EnsureSureWeaponNameIsSet`)
      (`self.EnsureWeaponHas >=1 AvailableFireModes`)
      (`self.EnsurePresetFireModeIsAnAvailableOne`)
      (`self.SetWeaponCosmetics`)
      (`self.UpdateArrowLocations`))
    (:`then_2`
      (`self.I_Reload`)
      (bind _pchar (message `/Game/FPSFramework/Blueprints/Characters/Player/I_PChar.I_GetPChar` (`self.GetOwner`)))
      (message `/Game/FPSFramework/UI/Blueprints/BPI_UI.I_UpdateFullWeaponUI` (`/Game/FPSFramework/Blueprints/Characters/Player/FirstPersonCharacter.HUDRef` _pchar)))))

(event `/Game/FPSFramework/Blueprints/Weapons/BPI_Weapons.I_Reload`
  (bind ((`AmmoType_6_45344AF441063A5C9476E5888D063293` _ammotype) (`MagazineSize_7_5536738D437728B3C178858506D7344E` _magazinesize)) (break `/Game/FPSFramework/Blueprints/Structs/WpnAmmoPropertiesStruct` (`.AmmoProperties_25_2065D3814E43080D3DBE0D9C85ED7188` (break `/Game/FPSFramework/Blueprints/Structs/FullWpnPropertiesStruct` (`self.WeaponProperties`)))))
  ;[1 1 1] Reload
  (`KismetSystemLibrary.PrintString` "Reloading...")
  (set `self.IsReloading?` true)
  (bind _amountheld (message `/Game/FPSFramework/Blueprints/Characters/Player/BPI_Inventory.I_GetAmmo` (`self.GetOwner`) _ammotype))
  (if (>= _amountheld _magazinesize)
    (set `self.AmmoLeftInMag` _magazinesize)
    (else
      (set `self.AmmoLeftInMag` _amountheld)))
  (bind _pchar (message `/Game/FPSFramework/Blueprints/Characters/Player/I_PChar.I_GetPChar` (`self.GetOwner`)))
  (message `/Game/FPSFramework/UI/Blueprints/BPI_UI.I_UpdateAmmoUI` (`/Game/FPSFramework/Blueprints/Characters/Player/FirstPersonCharacter.HUDRef` _pchar))
  (set `self.IsReloading?` false))

(event `CallSingleFire`
  ;[1 1 1] Single Fire
  (bind (_canfire_ _reason_for_cannot_fire) (`self.CanFireWeapon`))
  (if _canfire_
    (`self.FireShot`)
    (else
      (`self.DisplayCannotFireReason` _reason_for_cannot_fire))))

(event `/Game/FPSFramework/Blueprints/Weapons/BPI_Weapons.I_PrimaryFire`
  ;[1 1 1] Fire and Cancel Fire
  (if (not (`self.IsReloading?`))
    (switch `/Game/FPSFramework/Blueprints/Enumns/EWeaponFireModes` (`.CurrentFireMode_18_07D522D44AD946FCA01268AF4B035FBF` (break `/Game/FPSFramework/Blueprints/Structs/WpnBasePropertiesStruct` (`.Base_3_D073CF5543E6666FFE3FC3AA1266B303` (break `/Game/FPSFramework/Blueprints/Structs/FullWpnPropertiesStruct` (`self.WeaponProperties`)))))
      (:`NewEnumerator0`
        (`self.CallSingleFire`))
      (:`NewEnumerator1`
        (`self.CallBurstFire`))
      (:`NewEnumerator2`
        (`self.CallAutoFire`)))))

(event `CallBurstFire`
  ;[1 1 1] BurstFire
  (if (not (`self.BurstFireActive`))
    (set `self.BurstFireActive` true)
    (`self.BurstFire`)
    (bind _returnvalue (`KismetSystemLibrary.K2_SetTimerDelegate` (delegate `BurstFire`) (`.Interval_6_9154511B4E8C0958086FAEB8C2A36BC8` (break `/Game/FPSFramework/Blueprints/Structs/WpnBurstFirePropertiesStruct` (`.BurstProperties_9_7E9DC268475A61DDB2B2FEBA379D6878` (break `/Game/FPSFramework/Blueprints/Structs/FullWpnPropertiesStruct` (`self.WeaponProperties`))))) true))
    (set `self.BurstFireTimerH` _returnvalue)))

(event `FireShot`
  (bind (_startloc _endloc _shotrotation) (`self.GetShotDirection`))
  (bind ((`Base_3_D073CF5543E6666FFE3FC3AA1266B303` _base) (`ShotProperties_5_B2456A4E4A519B70A4BC02AC05AC033C` _shotproperties)) (break `/Game/FPSFramework/Blueprints/Structs/FullWpnPropertiesStruct` (`self.WeaponProperties`)))
  (bind ((`WeaponType_11_6B093A2A461A079109DAA299A7B6A7B5` _weapontype) (`BaseDamagePerShot_21_F277489442F1CB5A05C358AC97BD8DF5` _basedamagepershot)) (break `/Game/FPSFramework/Blueprints/Structs/WpnBasePropertiesStruct` _base))
  (bind ((`PelletsPerShot_4_11A740B443B4BE6E2D9494931235F6F2` _pelletspershot) (`Projectile_8_56D225954FEB240BF20B0DBE7F0AE76B` _projectile) (`ProjectileMuzzleSpeed_11_49BBA3B14632ADFBB4DABC9FA4CD079D` _projectilemuzzlespeed)) (break `/Game/FPSFramework/Blueprints/Structs/WpnShotPropertiesStruct` _shotproperties))
  ;[1 1 1] Actual Shot Fire
  (for _ (range 1 (+ _pelletspershot 1))
    (switch `/Game/FPSFramework/Blueprints/Enumns/EWeaponTypes` _weapontype
      (:`NewEnumerator5`
        (bind _outhit (`KismetSystemLibrary.LineTraceSingle` :`Start` _startloc :`End` _endloc :`TraceChannel` "TraceTypeQuery1" :`DrawTime` 1.0))
        (bind (_bblockinghit _binitialoverlap _time _distance _location _impactpoint _normal _impactnormal _physmat _hitactor _hitcomponent _hitbonename _bonename _hititem _elementindex _faceindex _tracestart _traceend) (`GameplayStatics.BreakHitResult` _outhit))
        (`GameplayStatics.ApplyDamage` _hitactor _basedamagepershot (`Pawn.GetController` (`self.GetProjectileInstigator` (`self.GetOwner`))) self)
        (bind _returnvalue (`NiagaraFunctionLibrary.SpawnSystemAtLocation` (`.BeamFX_10_54DF54614EB1F73A6EFAF599CF50FD21` (break `/Game/FPSFramework/Blueprints/Structs/WpnCosmeticsStruct` (`.CosmeticProperties_28_7D9154E7427EC37259C88C9C3DAB187E` (break `/Game/FPSFramework/Blueprints/Structs/FullWpnPropertiesStruct` (`self.WeaponProperties`))))) _tracestart))
        (`NiagaraComponent.SetVariableVec3` _returnvalue "Beam End" (`KismetMathLibrary.SelectVector` _impactpoint _traceend _bblockinghit)))
      (:`NewEnumerator6`
        (bind _outhits (`KismetSystemLibrary.LineTraceMultiForObjects` _startloc _endloc (`|MakeArray` "ObjectTypeQuery1" "ObjectTypeQuery2" "ObjectTypeQuery3" :!type "EObjectTypeQuery Enum")))
        (for _array_element _outhits
          (`GameplayStatics.ApplyDamage` (`.HitActor` (`GameplayStatics.BreakHitResult` _array_element)) _basedamagepershot (`Pawn.GetController` (`self.GetProjectileInstigator` (`self.GetOwner`))) self))
        (bind (_bblockinghit_2 _binitialoverlap_2 _time_2 _distance_2 _location_2 _impactpoint_2 _normal_2 _impactnormal_2 _physmat_2 _hitactor_2 _hitcomponent_2 _hitbonename_2 _bonename_2 _hititem_2 _elementindex_2 _faceindex_2 _tracestart_2 _traceend_2) (`GameplayStatics.BreakHitResult` (`|GetArrayItem` _outhits)))
        (bind _returnvalue_2 (`NiagaraFunctionLibrary.SpawnSystemAtLocation` (`.BeamFX_10_54DF54614EB1F73A6EFAF599CF50FD21` (break `/Game/FPSFramework/Blueprints/Structs/WpnCosmeticsStruct` (`.CosmeticProperties_28_7D9154E7427EC37259C88C9C3DAB187E` (break `/Game/FPSFramework/Blueprints/Structs/FullWpnPropertiesStruct` (`self.WeaponProperties`))))) _tracestart_2))
        (`NiagaraComponent.SetVariableVec3` _returnvalue_2 "Beam End" _traceend_2))
      (:`NewEnumerator7`
        (`|SpawnActorFromClass` _projectile (`KismetMathLibrary.MakeTransform` _startloc _shotrotation) "Undefined" "SelectDefaultAtRuntime" self _projectilemuzzlespeed _basedamagepershot (`self.GetProjectileInstigator` (`self.GetOwner`))))))
  (`self.ApplyRecoil`)
  (`self.ReduceAmmo`)
  (`self.PlayFX`))

(event `/Game/FPSFramework/Blueprints/Weapons/BPI_Weapons.I_CancelPrimaryFire`
  ;[1 1 1] Fire and Cancel Fire
  (`KismetSystemLibrary.K2_ClearAndInvalidateTimerHandle` (`self.AutoFireTimerH`)))

(event `BurstFire`
  ;[1 1 1] BurstFire
  (bind (_canfire_ _reason_for_cannot_fire) (`self.CanFireWeapon`))
  (if _canfire_
    (`self.FireShot`)
    (bind _result (`/Engine/EditorBlueprintResources/StandardMacros.IncrementInt` (`self.CurrentBurstShot`))
      (:`  `
        (if (>= _result (`.MaxShotCount_5_4C9171E14862B4372DD9959AD1E009F9` (break `/Game/FPSFramework/Blueprints/Structs/WpnBurstFirePropertiesStruct` (`.BurstProperties_9_7E9DC268475A61DDB2B2FEBA379D6878` (break `/Game/FPSFramework/Blueprints/Structs/FullWpnPropertiesStruct` (`self.WeaponProperties`))))))
          (`KismetSystemLibrary.K2_ClearAndInvalidateTimerHandle` (`self.BurstFireTimerH`))
          (set `self.CurrentBurstShot` 0)
          (set `self.BurstFireActive` false))))
    (else
      (`self.DisplayCannotFireReason` _reason_for_cannot_fire)
      (`KismetSystemLibrary.K2_ClearAndInvalidateTimerHandle` (`self.BurstFireTimerH`))
      (set `self.CurrentBurstShot` 0)
      (set `self.BurstFireActive` false))))

(event `/Game/FPSFramework/Blueprints/Weapons/BPI_Weapons.I_SwitchFireMode`
  (bind ((`Base_3_D073CF5543E6666FFE3FC3AA1266B303` _base)) (break `/Game/FPSFramework/Blueprints/Structs/FullWpnPropertiesStruct` (`self.WeaponProperties`)))
  (bind ((`CurrentFireMode_18_07D522D44AD946FCA01268AF4B035FBF` _currentfiremode) (`AvailableFireModes_16_1D7D4F474D72565B56E64FBD8D84CE9B` _availablefiremodes)) (break `/Game/FPSFramework/Blueprints/Structs/WpnBasePropertiesStruct` _base))
  ;[1 1 1] Change Fire Mode
  (switch `/Game/FPSFramework/Blueprints/Enumns/EWeaponFireModes` _currentfiremode
    (:`NewEnumerator0`
      (setmembers `/Game/FPSFramework/Blueprints/Structs/WpnBasePropertiesStruct` :`StructRef` _base :`CurrentFireMode` "NewEnumerator1")
      (if (`BlueprintMapLibrary.Map_Find` _availablefiremodes _currentfiremode)
        (bind _pchar (message `/Game/FPSFramework/Blueprints/Characters/Player/I_PChar.I_GetPChar` (`self.GetOwner`) :!label _label))
        (message `/Game/FPSFramework/UI/Blueprints/BPI_UI.I_UpdateFireModeUI` (`/Game/FPSFramework/Blueprints/Characters/Player/FirstPersonCharacter.HUDRef` _pchar))
        (else
          (`self.I_SwitchFireMode` :!label _label_2))))
    (:`NewEnumerator1`
      (setmembers `/Game/FPSFramework/Blueprints/Structs/WpnBasePropertiesStruct` :`StructRef` _base :`CurrentFireMode` "NewEnumerator2")
      (if (`BlueprintMapLibrary.Map_Find` _availablefiremodes _currentfiremode)
        (goto _label)
        (else
          (goto _label_2))))
    (:`NewEnumerator2`
      (setmembers `/Game/FPSFramework/Blueprints/Structs/WpnBasePropertiesStruct` :`StructRef` _base :`CurrentFireMode` "NewEnumerator0")
      (if (`BlueprintMapLibrary.Map_Find` _availablefiremodes _currentfiremode)
        (goto _label)
        (else
          (goto _label_2))))))

(event `CallAutoFire`
  ;[1 1 1] Fully Automatic Fire
  (`self.AutoFire`)
  (bind _returnvalue (`KismetSystemLibrary.K2_SetTimerDelegate` (delegate `AutoFire`) (`.AutomaticFireInterval_15_02F181514C4DF8A36F1F689425E43E7A` (break `/Game/FPSFramework/Blueprints/Structs/FullWpnPropertiesStruct` (`self.WeaponProperties`))) true))
  (set `self.AutoFireTimerH` _returnvalue))

(event `ApplyRecoil`
  (bind _returnvalue (`Controller.K2_GetPawn` (`GameplayStatics.GetPlayerController` 0)))
  (bind (_minvertical _maxvertical _minhorizontal _maxhorizontal) (break `/Game/FPSFramework/Blueprints/Structs/WpnRecoilPropertiesStruct` (`.RecoilProperties_16_AC71A6A84A294380B7DD5596F5B3F4A6` (break `/Game/FPSFramework/Blueprints/Structs/FullWpnPropertiesStruct` (`self.WeaponProperties`)))))
  ;[1 1 1] Recoil
  (`Pawn.AddControllerPitchInput` _returnvalue (`KismetMathLibrary.RandomFloatInRange` _maxvertical _minvertical))
  (`Pawn.AddControllerYawInput` _returnvalue (`KismetMathLibrary.RandomFloatInRange` _minhorizontal _maxhorizontal)))

(event `ReduceAmmo`
  (bind ((`AmmoType_6_45344AF441063A5C9476E5888D063293` _ammotype) (`AmmoUsedPerShot_8_4E2CCC1E475F94EE0D38E9AE3E7B2DC7` _ammousedpershot)) (break `/Game/FPSFramework/Blueprints/Structs/WpnAmmoPropertiesStruct` (`.AmmoProperties_25_2065D3814E43080D3DBE0D9C85ED7188` (break `/Game/FPSFramework/Blueprints/Structs/FullWpnPropertiesStruct` (`self.WeaponProperties`)))))
  ;[1 1 1] Reduce Ammo
  (set `self.AmmoLeftInMag` (- (`self.AmmoLeftInMag`) _ammousedpershot))
  (message `/Game/FPSFramework/Blueprints/Characters/Player/BPI_Inventory.I_UpdateStoredAmmo` (`self.GetOwner`) _ammotype (* _ammousedpershot -1))
  (bind _pchar (message `/Game/FPSFramework/Blueprints/Characters/Player/I_PChar.I_GetPChar` (`self.GetOwner`)))
  (message `/Game/FPSFramework/UI/Blueprints/BPI_UI.I_UpdateAmmoUI` (`/Game/FPSFramework/Blueprints/Characters/Player/FirstPersonCharacter.HUDRef` _pchar)))

(event `AutoFire`
  ;[1 1 1] Fully Automatic Fire
  (bind (_canfire_ _reason_for_cannot_fire) (`self.CanFireWeapon`))
  (if _canfire_
    (`self.FireShot`)
    (else
      (`self.DisplayCannotFireReason` _reason_for_cannot_fire)
      (`KismetSystemLibrary.K2_ClearAndInvalidateTimerHandle` (`self.AutoFireTimerH`)))))

(event `/Game/FPSFramework/Blueprints/Weapons/BPI_Weapons.I_SetIsInADS`
  (params (IsInADS :type Boolean))
  ;[1 1 1] Set IsInADS
  (set `self.IsInADS?` IsInADS))

(event `PlayFX`
  (bind _returnvalue (`SceneComponent.K2_GetComponentLocation` (`self.FirePoint`)))
  ;[1 1 1] FX - Camera Shakes, Sound, Extra Particles
  (`GameplayStatics.PlayWorldCameraShake` "/Game/FPSFramework/Blueprints/CameraShakes/WeaponFire.WeaponFire_C" _returnvalue 0.1 1000.0 0.0 true)
  (`GameplayStatics.PlaySoundAtLocation` "/Game/FPSFramework/Audio/WeaponFire_Cue.WeaponFire_Cue" _returnvalue (struct) 1.0 1.0 0.0 null null null null))

(fn `CanFireWeapon`
  (returns (`CanFire?` :type Boolean) (`Reason For Cannot Fire` :type String))
  (if (>= (`self.AmmoLeftInMag`) (`.AmmoUsedPerShot_8_4E2CCC1E475F94EE0D38E9AE3E7B2DC7` (break `/Game/FPSFramework/Blueprints/Structs/WpnAmmoPropertiesStruct` (`.AmmoProperties_25_2065D3814E43080D3DBE0D9C85ED7188` (break `/Game/FPSFramework/Blueprints/Structs/FullWpnPropertiesStruct` (`self.WeaponProperties`))))))
    (return true "")
    (else
      (return false "Not enough ammo in magazine"))))

(fn `DisplayCannotFireReason`
  (params (Selection :type String))
  (switch `string` Selection
    (:`Default`
      (`KismetSystemLibrary.PrintString` "No reason provided for failure to fire" true true (struct :`R` 1.0 :`B` 0.082138 :`A` 1.0)))
    (:`Not enough ammo in magazine`
      (bind _pchar (message `/Game/FPSFramework/Blueprints/Characters/Player/I_PChar.I_GetPChar` (`self.GetOwner`)))
      (message `/Game/FPSFramework/UI/Blueprints/BPI_UI.I_ShowNoAmmoWarning` (`/Game/FPSFramework/Blueprints/Characters/Player/FirstPersonCharacter.HUDRef` _pchar)))))

(fn `EnsurePresetFireModeIsAnAvailableOne`
  (bind ((`CurrentFireMode_18_07D522D44AD946FCA01268AF4B035FBF` _currentfiremode) (`AvailableFireModes_16_1D7D4F474D72565B56E64FBD8D84CE9B` _availablefiremodes)) (break `/Game/FPSFramework/Blueprints/Structs/WpnBasePropertiesStruct` (`.Base_3_D073CF5543E6666FFE3FC3AA1266B303` (break `/Game/FPSFramework/Blueprints/Structs/FullWpnPropertiesStruct` (`self.WeaponProperties`)))))
  ;[1 1 1] If preset current fire mode is unavialable, set weapon to first available mode
  (if (not (`BlueprintMapLibrary.Map_Find` _availablefiremodes _currentfiremode))
    (bind _keys (`BlueprintMapLibrary.Map_Keys` _availablefiremodes))
    (for _array_element _keys
      (if (`BlueprintMapLibrary.Map_Find` _availablefiremodes _array_element)
        (setmembers `/Game/FPSFramework/Blueprints/Structs/WpnBasePropertiesStruct` :`StructRef` (`.Base_3_D073CF5543E6666FFE3FC3AA1266B303` (break `/Game/FPSFramework/Blueprints/Structs/FullWpnPropertiesStruct` (`self.WeaponProperties`))) :`CurrentFireMode` _array_element)
        (break))))
  (return))

(fn `EnsureSureWeaponNameIsSet`
  (bind ((`Base_3_D073CF5543E6666FFE3FC3AA1266B303` _base)) (break `/Game/FPSFramework/Blueprints/Structs/FullWpnPropertiesStruct` (`self.WeaponProperties`)))
  (if (`KismetStringLibrary.IsEmpty` (`.WeaponName_10_FDF25DFF4A74F28E1B3373B06C1E3D59` (break `/Game/FPSFramework/Blueprints/Structs/WpnBasePropertiesStruct` _base)))
    (setmembers `/Game/FPSFramework/Blueprints/Structs/WpnBasePropertiesStruct` :`StructRef` _base :`WeaponName` (`KismetSystemLibrary.GetClassDisplayName` (`GameplayStatics.GetObjectClass` self))))
  (return))

(fn `EnsureWeaponHas >=1 AvailableFireModes`
  (locals (`Has>=1AvailableFireModes` :type Boolean))
  (bind ((`AvailableFireModes_16_1D7D4F474D72565B56E64FBD8D84CE9B` _availablefiremodes)) (break `/Game/FPSFramework/Blueprints/Structs/WpnBasePropertiesStruct` (`.Base_3_D073CF5543E6666FFE3FC3AA1266B303` (break `/Game/FPSFramework/Blueprints/Structs/FullWpnPropertiesStruct` (`self.WeaponProperties`)))))
  ;[1 1 1] If weapon has no available fire modes, give it single fire
  (bind _values (`BlueprintMapLibrary.Map_Values` _availablefiremodes))
  (for _array_element _values
    (if _array_element
      (set `local.Has>=1AvailableFireModes` true)
      (break)
      (else
        (set `local.Has>=1AvailableFireModes` false))))
  (if (not (`local.Has>=1AvailableFireModes`))
    (`BlueprintMapLibrary.Map_Add` _availablefiremodes "NewEnumerator0" true))
  (return))

(fn `GetProjectileInstigator`
  (params (WeaponParentActor :type "Object Object Reference"))
  (returns (PChar :type "/Game/FPSFramework/Blueprints/Characters/Player/FirstPersonCharacter Object Reference"))
  (bind _pchar (message `/Game/FPSFramework/Blueprints/Characters/Player/I_PChar.I_GetPChar` WeaponParentActor))
  (return _pchar))

(fn `GetShotDirection`
  (returns (StartLoc :type "Vector Structure") (EndLoc :type "Vector Structure") (ShotRotation :type "Rotator Structure"))
  (locals (NewLocalVar_0 :type "Float (double-precision)" :default 5.0))
  (bind ((`Base_3_D073CF5543E6666FFE3FC3AA1266B303` _base) (`ShotProperties_5_B2456A4E4A519B70A4BC02AC05AC033C` _shotproperties)) (break `/Game/FPSFramework/Blueprints/Structs/FullWpnPropertiesStruct` (`self.WeaponProperties`)))
  (bind _returnvalue (`SceneComponent.K2_GetComponentLocation` (`self.FirePoint`)))
  (bind (_x _y) (`KismetMathLibrary.BreakVector2D` (`WidgetLayoutLibrary.GetViewportSize`)))
  (bind ((`Innacuracy_5_504ADB0A4F7FC46A5A4D3D8D1A464834` _innacuracy) (`ADSInnacuracyMultiplier_14_60D1D6B14DC69DA29B8982BF00252E91` _adsinnacuracymultiplier)) (break `/Game/FPSFramework/Blueprints/Structs/WpnShotPropertiesStruct` _shotproperties))
  (bind _returnvalue_2 (+ (`GameplayStatics.DeprojectScreenToWorld` (`GameplayStatics.GetPlayerController` 0) (`KismetMathLibrary.MakeVector2D` (/ _x 2.0) (/ _y 2.0))) (* (`KismetMathLibrary.RandomUnitVectorInConeInDegrees` (`self.GetActorForwardVector` (`GameplayStatics.GetPlayerCameraManager` 0)) (`KismetMathLibrary.SelectFloat` _innacuracy (* _innacuracy _adsinnacuracymultiplier) (not (`self.IsInADS?`)))) (`.MaxEffectiveRange_17_A094F36E4174BC7BE829E3ACD73EC745` (break `/Game/FPSFramework/Blueprints/Structs/WpnBasePropertiesStruct` _base)))))
  (return _returnvalue _returnvalue_2 (`KismetMathLibrary.FindLookAtRotation` _returnvalue _returnvalue_2)))

(fn `I_GetAmmoInGun`
  (returns (AmmoInMag :type Integer) (MagSize :type Integer) (AmmoType :type "/Game/FPSFramework/Blueprints/Enumns/EAmmoTypes Enum"))
  (bind ((`AmmoType_6_45344AF441063A5C9476E5888D063293` _ammotype) (`MagazineSize_7_5536738D437728B3C178858506D7344E` _magazinesize)) (break `/Game/FPSFramework/Blueprints/Structs/WpnAmmoPropertiesStruct` (`.AmmoProperties_25_2065D3814E43080D3DBE0D9C85ED7188` (break `/Game/FPSFramework/Blueprints/Structs/FullWpnPropertiesStruct` (`self.WeaponProperties`)))))
  (return (`self.AmmoLeftInMag`) _magazinesize _ammotype))

(fn `I_GetCurrentFireMode`
  (returns (FireMode :type "/Game/FPSFramework/Blueprints/Enumns/EWeaponFireModes Enum"))
  (return (`.CurrentFireMode_18_07D522D44AD946FCA01268AF4B035FBF` (break `/Game/FPSFramework/Blueprints/Structs/WpnBasePropertiesStruct` (`.Base_3_D073CF5543E6666FFE3FC3AA1266B303` (break `/Game/FPSFramework/Blueprints/Structs/FullWpnPropertiesStruct` (`self.WeaponProperties`)))))))

(fn `I_GetWeapon`
  (returns (Weapon :type "/Game/FPSFramework/Blueprints/Weapons/BP_BaseGun Object Reference"))
  (return self))

(fn `SetWeaponCosmetics`
  (`SkinnedMeshComponent.SetSkinnedAssetAndUpdate` (`self.SkeletalMesh`) (`.SkeleMesh_4_5C12C40B4E44497C4CA002AEAC24959B` (break `/Game/FPSFramework/Blueprints/Structs/WpnCosmeticsStruct` (`.CosmeticProperties_28_7D9154E7427EC37259C88C9C3DAB187E` (break `/Game/FPSFramework/Blueprints/Structs/FullWpnPropertiesStruct` (`self.WeaponProperties`))))) true))

(fn `UpdateArrowLocations`
  (bind _skeletalmesh (`self.SkeletalMesh`))
  (`SceneComponent.K2_SetWorldLocation` (`self.FirePoint`) (`SceneComponent.GetSocketLocation` _skeletalmesh "Muzzle") false false)
  (`SceneComponent.K2_SetWorldLocation` (`self.SightsView`) (`SceneComponent.GetSocketLocation` _skeletalmesh "IronSights") false false))

(fn `UserConstructionScript`)